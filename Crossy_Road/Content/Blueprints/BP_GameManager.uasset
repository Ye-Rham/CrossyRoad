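; Game manager actor that runs session setup, HUD and the auto-scrolling camera for what appears to be a tile-based hopper game.
; On BeginPlay it resets step and coin counters, becomes the view target, creates WBP_UI and spawns BP_TileSpawner to lay the initial tiles, handing both a back-reference.
; Tick creeps the camera along Y and Z, snaps it forward in Y when the player gets too far ahead, and follows the player in X within set bounds.
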(event EventBeginPlay
  (CallFunction|ResetStats)
  (CallFunction|SetUpCamera)
  (bind _returnvalue (UserInterface|CreateWidget "/Game/Blueprints/WBP_UI.WBP_UI_C"))
  (UserInterface|Viewport|AddtoViewport _returnvalue 0)
  (Variables|/Game/Blueprints/WBP_UI.WBP_UI_C|SetBP_GameManager _returnvalue self)
  (bind _output_get (Variables|Default|SetHUD _returnvalue))
  (Default|UpdateCounter _output_get)
  (Default|UpdateCoins _output_get)
  (bind _returnvalue_2 (Game|SpawnActorfromClass "/Game/Blueprints/BP_TileSpawner.BP_TileSpawner_C" (Math|Transform|MakeTransform "0, 0, 0" "0, 0, 0" "1,1,1") "Undefined" 0 0))
  (Variables|/Game/Blueprints/BP_TileSpawner.BP_TileSpawner_C|SetBP_GameManager _returnvalue_2 self)
  (Default|SpawnInitialTiles _returnvalue_2))

(event Collision|EventActorBeginOverlap
  (params (OtherActor :type Actor%20Object%20Reference)))

(event EventTick
  (params (DeltaSeconds :type Float%20%28single-precision%29))
  (bind _returnvalue (Game|Player|GetPlayerPawn 0))
  (bind _returnvalue_2 (* DeltaSeconds -2e+01))
  (bind _returnvalue_3 (* DeltaSeconds 1e+01))
  (bind _camera (Variables|Default|GetCamera))
  (bind _camera_2 (Variables|Default|GetCamera))
  (bind _camera_3 (Variables|Default|GetCamera))
  (bind _returnvalue_4 (Transformation|GetActorLocation _returnvalue))
  (bind _returnvalue_5 (Transformation|GetWorldLocation _camera_2))
  (Transformation|AddLocalOffset _camera (Math|Vector|MakeVector 0.0 _returnvalue_3 _returnvalue_3) false false)
  (if (> (- (.y _returnvalue_4) (.y _returnvalue_5)) 7.2e+02)
    (Transformation|AddLocalOffset _camera (Math|Vector|MakeVector 0.0 _returnvalue_2 _returnvalue_2) false false)
    (Transformation|SetWorldLocation _camera_3 (Math|Vector|MakeVector (.x _returnvalue_5) (- (.y _returnvalue_4) 7.2e+02) (.z _returnvalue_5)) false false))
  (if (and (> (- (.x _returnvalue_4) (.x _returnvalue_5)) 3.2e+02) (<= (.x _returnvalue_4) 2.4e+02))
    (Transformation|SetWorldLocation _camera_3 (Math|Vector|MakeVector (- (.x _returnvalue_4) 3.2e+02) (.y _returnvalue_5) (.z _returnvalue_5)) false false)
    (elif (and (< (- (.x _returnvalue_4) (.x _returnvalue_5)) 3.2e+02) (>= (.x _returnvalue_4) -2.4e+02))
      (Transformation|SetWorldLocation _camera_3 (Math|Vector|MakeVector (- (.x _returnvalue_4) 3.2e+02) (.y _returnvalue_5) (.z _returnvalue_5)) false false))))

(fn ConstructionScript)

(fn ResetStats
  (Variables|Default|SetStepCounter 0)
  (Variables|Default|SetCoinCounter 0))

(fn SetUpCamera
  (Game|Player|SetViewTargetwithBlend (Game|GetPlayerController 0) self 0.0 "VTBlend_Linear" 0.0 false))