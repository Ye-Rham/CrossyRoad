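; Player chicken that hops one grid cell at a time in four directions, Crossy Road style.
; Holding a direction squashes the mesh; release rotates it and launches a hop, unless that neighbour is flagged in the next, previous or current row arrays.
; Tick moves the actor by consumed movement input, pulling Direction downward for an arc.
; After a short delay with input disabled, it snaps to the target cell.
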(event EventBeginPlay)

(event Collision|EventActorBeginOverlap
  (params (OtherActor :type Actor%20Object%20Reference)))

(event EventTick
  (params (DeltaSeconds :type Float%20%28single-precision%29))
  (Pawn|Input|AddMovementInput (Variables|Default|GetDirection) (Variables|Default|GetSpeed) false)
  (bind _returnvalue (Class|Pawn|ConsumeMovementInputVector))
  (Transformation|AddActorLocalOffset (* _returnvalue DeltaSeconds) false false)
  (if (Variables|Default|GetMoving)
    (Variables|Default|SetDirection (+ (Variables|Default|GetDirection) (* "0, 0,-16.000000" DeltaSeconds))))
  (CallFunction|Shrink))

(event Input|ActionEvents|InputActionForward
  (params (Key :type Key%20Structure))
  (bind _returnvalue (Transformation|GetActorLocation))
  (bind _currentposition (Variables|Default|GetCurrentPosition))
  (bind _nextobjects (Variables|Default|GetNextObjects))
  (bind _staticmesh (Variables|Default|GetStaticMesh))
  (bind _output (Utilities|Array|Get(acopy) _nextobjects _currentposition))
  (:Pressed
    (if (not _output)
      (Variables|Default|SetShrinking true)))
  (:Released
    (if (not _output)
      (Input|DisableInput 0)
      (Transformation|SetWorldRotation _staticmesh "0, 0, 0" false false)
      (Variables|Default|SetDirection "0.0,1.0,2.000000")
      (Variables|Default|SetFinalLocation (Math|Vector|MakeVector (.x _returnvalue) (+ (.y _returnvalue) 8e+01) 15.0))
      (Variables|Default|SetMoving true)
      (Variables|Default|SetShrinking false)
      (bind _output_get (Variables|Default|SetScale "1.000000,1.000000,1.000000"))
      (Transformation|SetRelativeScale3D _staticmesh _output_get)
      (Utilities|FlowControl|Delay 0.25)
      (Variables|Default|SetMoving false)
      (Variables|Default|SetDirection "0, 0, 0")
      (Transformation|SetActorLocation (Variables|Default|GetFinalLocation) false false)
      (Input|EnableInput 0))))

(event Input|ActionEvents|InputActionBackward
  (params (Key :type Key%20Structure))
  (bind _returnvalue (Transformation|GetActorLocation))
  (bind _currentposition (Variables|Default|GetCurrentPosition))
  (bind _previousobjects (Variables|Default|GetPreviousObjects))
  (bind _staticmesh (Variables|Default|GetStaticMesh))
  (bind _output (Utilities|Array|Get(acopy) _previousobjects _currentposition))
  (:Pressed
    (if (not _output)
      (Variables|Default|SetShrinking true)))
  (:Released
    (if (not _output)
      (Input|DisableInput 0)
      (Transformation|SetWorldRotation _staticmesh "0,180.000000, 0" false false)
      (Variables|Default|SetDirection "0,-1.000000,2.000000")
      (Variables|Default|SetFinalLocation (Math|Vector|MakeVector (.x _returnvalue) (+ (.y _returnvalue) -8e+01) 15.0))
      (Variables|Default|SetMoving true)
      (Variables|Default|SetShrinking false)
      (bind _output_get (Variables|Default|SetScale "1.000000,1.000000,1.000000"))
      (Transformation|SetRelativeScale3D _staticmesh _output_get)
      (Utilities|FlowControl|Delay 0.25)
      (Variables|Default|SetMoving false)
      (Variables|Default|SetDirection "0, 0, 0")
      (Transformation|SetActorLocation (Variables|Default|GetFinalLocation) false false)
      (Input|EnableInput 0))))

(event Input|ActionEvents|InputActionRight
  (params (Key :type Key%20Structure))
  (bind _returnvalue (Transformation|GetActorLocation))
  (bind _currentobjects (Variables|Default|GetCurrentObjects))
  (bind _currentposition (Variables|Default|GetCurrentPosition))
  (bind _staticmesh (Variables|Default|GetStaticMesh))
  (bind _returnvalue_2 (+ _currentposition 1))
  (bind _output (Utilities|Array|Get(acopy) _currentobjects _returnvalue_2))
  (:Pressed
    (if (not _output)
      (Variables|Default|SetShrinking true)))
  (:Released
    (if (not _output)
      (Math|Integer|IncrementInt _currentposition
        (:%20%20
          (Input|DisableInput 0)
          (Transformation|SetWorldRotation _staticmesh "0,90.000000, 0" false false)
          (Variables|Default|SetDirection "-1.000000,0.000000,2.000000")
          (Variables|Default|SetFinalLocation (Math|Vector|MakeVector (+ (.x _returnvalue) -8e+01) (.y _returnvalue) 15.0))
          (Variables|Default|SetMoving true)
          (Variables|Default|SetShrinking false)
          (bind _output_get (Variables|Default|SetScale "1.000000,1.000000,1.000000"))
          (Transformation|SetRelativeScale3D _staticmesh _output_get)
          (Utilities|FlowControl|Delay 0.25)
          (Variables|Default|SetMoving false)
          (Variables|Default|SetDirection "0, 0, 0")
          (Transformation|SetActorLocation (Variables|Default|GetFinalLocation) false false)
          (Input|EnableInput 0))))))

(event Input|ActionEvents|InputActionLeft
  (params (Key :type Key%20Structure))
  (bind _returnvalue (Transformation|GetActorLocation))
  (bind _currentobjects (Variables|Default|GetCurrentObjects))
  (bind _currentposition (Variables|Default|GetCurrentPosition))
  (bind _staticmesh (Variables|Default|GetStaticMesh))
  (bind _returnvalue_2 (- _currentposition 1))
  (bind _output (Utilities|Array|Get(acopy) _currentobjects _returnvalue_2))
  (:Pressed
    (if (not _output)
      (Variables|Default|SetShrinking true)))
  (:Released
    (if (not _output)
      (Math|Integer|DecrementInt _currentposition
        (:%20%20
          (Input|DisableInput 0)
          (Transformation|SetWorldRotation _staticmesh "0,-90.000000, 0" false false)
          (Variables|Default|SetDirection "1.000000, 0,2.000000")
          (Variables|Default|SetFinalLocation (Math|Vector|MakeVector (+ (.x _returnvalue) 8e+01) (.y _returnvalue) 15.0))
          (Variables|Default|SetMoving true)
          (Variables|Default|SetShrinking false)
          (bind _output_get (Variables|Default|SetScale "1.000000,1.000000,1.000000"))
          (Transformation|SetRelativeScale3D _staticmesh _output_get)
          (Utilities|FlowControl|Delay 0.25)
          (Variables|Default|SetMoving false)
          (Variables|Default|SetDirection "0, 0, 0")
          (Transformation|SetActorLocation (Variables|Default|GetFinalLocation) false false)
          (Input|EnableInput 0))))))

(fn ConstructionScript)

(fn Shrink
  (if (and (Variables|Default|GetShrinking) (> (.z (Variables|Default|GetScale)) 0.75))
    (bind _output_get (Variables|Default|SetScale (Math|Vector|MakeVector 1.0 1.0 (- (.z (Variables|Default|GetScale)) 0.05))))
    (Transformation|SetRelativeScale3D (Variables|Default|GetStaticMesh) _output_get))
  (return))