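; Tile spawner actor that lays out the opening chain of BP_Tile actors when play begins.
; It places pre-triggered forest tiles from just behind the player's Y position, then pre-triggered starting tiles, then tiles of the latest type.
; Each tile spawns at the newest tile's SpawnPoint and receives a reference to the spawner.
; Neighboring tiles exchange their Objects as previous and next links as the chain grows.
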(event EventBeginPlay
  (CallFunction|SpawnInitialTiles))

(event Collision|EventActorBeginOverlap
  (params (OtherActor :type Actor%20Object%20Reference)))

(event EventTick
  (params (DeltaSeconds :type Float%20%28single-precision%29)))

(fn ConstructionScript)

(fn SpawnTile
  (params (SpawnLocation :type Vector) (TileType :type String))
  (bind _returnvalue (Game|SpawnActorfromClass "/Game/Blueprints/BP_Tile.BP_Tile_C" (Math|Transform|MakeTransform SpawnLocation "0, 0, 0" "1,1,1") "Undefined" 0 0))
  (Variables|/Game/Blueprints/BP_Tile.BP_Tile_C|SetTileType _returnvalue TileType)
  (Variables|/Game/Blueprints/BP_Tile.BP_Tile_C|SetTileSpawner _returnvalue self)
  (Variables|/Game/Blueprints/BP_Tile.BP_Tile_C|SetPreviousObjects _returnvalue (Variables|Default|GetObjects))
  (Variables|Default|SetPreviousObjects (Variables|Default|GetObjects))
  (bind _tile (Default|MakeTile _returnvalue))
  (Utilities|IsValid (Variables|Default|GetNewestTile)
    (:Is%20Valid
      (Variables|/Game/Blueprints/BP_Tile.BP_Tile_C|SetNextObjects (Variables|Default|GetNewestTile) (Variables|/Game/Blueprints/BP_Tile.BP_Tile_C|GetObjects _tile)))
    (:Is%20Not%20Valid
      _))
  (bind _output_get (Variables|Default|SetNewestTile _tile))
  (Variables|Default|SetObjects (Variables|/Game/Blueprints/BP_Tile.BP_Tile_C|GetObjects _output_get)))

(fn SpawnTileatLocation
  (CallFunction|SpawnTile (Transformation|GetWorldLocation (Variables|/Game/Blueprints/BP_Tile.BP_Tile_C|GetSpawnPoint (Variables|Default|GetNewestTile))) (Variables|Default|GetLatestTileType)))

(fn SpawnInitialTiles
  (bind _returnvalue (Game|Player|GetPlayerPawn 0))
  (bind _returnvalue_2 (Transformation|GetActorLocation _returnvalue))
  (for _index (range 0 1)
    (Utilities|IsValid (Variables|Default|GetNewestTile)
      (:Is%20Valid
        (bind _returnvalue_3 (Game|SpawnActorfromClass "/Game/Blueprints/BP_Tile.BP_Tile_C" (Math|Transform|MakeTransform (Transformation|GetWorldLocation (Variables|/Game/Blueprints/BP_Tile.BP_Tile_C|GetSpawnPoint (Variables|Default|GetNewestTile))) "0, 0, 0" "1,1,1") "Undefined" 0 0))
        (Variables|/Game/Blueprints/BP_Tile.BP_Tile_C|SetTileType _returnvalue_3 (Variables|Default|GetLatestTileType))
        (Variables|/Game/Blueprints/BP_Tile.BP_Tile_C|SetTileSpawner _returnvalue_3 self)
        (Variables|/Game/Blueprints/BP_Tile.BP_Tile_C|SetPreviousObjects _returnvalue_3 (Variables|Default|GetObjects))
        (Variables|Default|SetPreviousObjects (Variables|Default|GetObjects))
        (bind _tile (Default|MakeForestTile _returnvalue_3))
        (Utilities|IsValid (Variables|Default|GetNewestTile)
          (:Is%20Valid
            (Variables|/Game/Blueprints/BP_Tile.BP_Tile_C|SetNextObjects (Variables|Default|GetNewestTile) (Variables|/Game/Blueprints/BP_Tile.BP_Tile_C|GetObjects _tile)))
          (:Is%20Not%20Valid
            _))
        (bind _output_get (Variables|Default|SetNewestTile _tile))
        (Variables|Default|SetObjects (Variables|/Game/Blueprints/BP_Tile.BP_Tile_C|GetObjects _output_get))
        (Variables|/Game/Blueprints/BP_Tile.BP_Tile_C|SetTriggered _tile true))
      (:Is%20Not%20Valid
        (bind _returnvalue_4 (Game|SpawnActorfromClass "/Game/Blueprints/BP_Tile.BP_Tile_C" (Math|Transform|MakeTransform (Math|Vector|MakeVector (.x _returnvalue_2) (- (.y _returnvalue_2) 3.2e+02) 0.0) "0, 0, 0" "1,1,1") "Undefined" 0 0))
        (Variables|/Game/Blueprints/BP_Tile.BP_Tile_C|SetTileType _returnvalue_4 (Variables|Default|GetLatestTileType))
        (Variables|/Game/Blueprints/BP_Tile.BP_Tile_C|SetTileSpawner _returnvalue_4 self)
        (Variables|/Game/Blueprints/BP_Tile.BP_Tile_C|SetPreviousObjects _returnvalue_4 (Variables|Default|GetObjects))
        (Variables|Default|SetPreviousObjects (Variables|Default|GetObjects))
        (bind _tile_2 (Default|MakeForestTile _returnvalue_4))
        (Utilities|IsValid (Variables|Default|GetNewestTile)
          (:Is%20Valid
            (Variables|/Game/Blueprints/BP_Tile.BP_Tile_C|SetNextObjects (Variables|Default|GetNewestTile) (Variables|/Game/Blueprints/BP_Tile.BP_Tile_C|GetObjects _tile_2)))
          (:Is%20Not%20Valid
            _))
        (bind _output_get_2 (Variables|Default|SetNewestTile _tile_2))
        (Variables|Default|SetObjects (Variables|/Game/Blueprints/BP_Tile.BP_Tile_C|GetObjects _output_get_2))
        (Variables|/Game/Blueprints/BP_Tile.BP_Tile_C|SetTriggered _tile_2 true))))
  (for _index_2 (range 0 3)
    (bind _returnvalue_5 (Game|SpawnActorfromClass "/Game/Blueprints/BP_Tile.BP_Tile_C" (Math|Transform|MakeTransform (Transformation|GetWorldLocation (Variables|/Game/Blueprints/BP_Tile.BP_Tile_C|GetSpawnPoint (Variables|Default|GetNewestTile))) "0, 0, 0" "1,1,1") "Undefined" 0 0))
    (Variables|/Game/Blueprints/BP_Tile.BP_Tile_C|SetTileType _returnvalue_5 (Variables|Default|GetLatestTileType))
    (Variables|/Game/Blueprints/BP_Tile.BP_Tile_C|SetTileSpawner _returnvalue_5 self)
    (Variables|/Game/Blueprints/BP_Tile.BP_Tile_C|SetPreviousObjects _returnvalue_5 (Variables|Default|GetObjects))
    (Variables|Default|SetPreviousObjects (Variables|Default|GetObjects))
    (bind _tile_3 (Default|MakeStartingTile _returnvalue_5))
    (Utilities|IsValid (Variables|Default|GetNewestTile)
      (:Is%20Valid
        (Variables|/Game/Blueprints/BP_Tile.BP_Tile_C|SetNextObjects (Variables|Default|GetNewestTile) (Variables|/Game/Blueprints/BP_Tile.BP_Tile_C|GetObjects _tile_3)))
      (:Is%20Not%20Valid
        _))
    (bind _output_get_3 (Variables|Default|SetNewestTile _tile_3))
    (Variables|Default|SetObjects (Variables|/Game/Blueprints/BP_Tile.BP_Tile_C|GetObjects _output_get_3))
    (Variables|/Game/Blueprints/BP_Tile.BP_Tile_C|SetTriggered _tile_3 true))
  (for _index_3 (range 0 14)
    (CallFunction|SpawnTileatLocation)))