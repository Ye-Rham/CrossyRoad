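; BP_Car is a car actor that drives in a straight line along its local X axis with a randomly chosen color.
; On BeginPlay, a random switch adds a static mesh component at runtime and assigns it the blue, green, orange or purple car mesh.
; Tick moves the actor by Speed scaled by delta time, keeping movement frame-rate independent.
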(event EventBeginPlay
  (switch int (Math|Random|RandomInteger 4)
    (:0
      (bind _returnvalue (AddComponent|AddStaticMeshComponent false))
      (Components|StaticMesh|SetStaticMesh _returnvalue "/Game/Meshes/BlueCar.BlueCar"))
    (:1
      (bind _returnvalue_2 (AddComponent|AddStaticMeshComponent false))
      (Components|StaticMesh|SetStaticMesh _returnvalue_2 "/Game/Meshes/GreenCar.GreenCar"))
    (:2
      (bind _returnvalue_3 (AddComponent|AddStaticMeshComponent false))
      (Components|StaticMesh|SetStaticMesh _returnvalue_3 "/Game/Meshes/OrangeCar.OrangeCar"))
    (:3
      (bind _returnvalue_4 (AddComponent|AddStaticMeshComponent false))
      (Components|StaticMesh|SetStaticMesh _returnvalue_4 "/Game/Meshes/PurpleCar.PurpleCar"))))

(event Collision|EventActorBeginOverlap
  (params (OtherActor :type Actor%20Object%20Reference)))

(event EventTick
  (params (DeltaSeconds :type Float%20%28single-precision%29))
  (Transformation|AddActorLocalOffset (Math|Vector|MakeVector (* DeltaSeconds (Variables|Default|GetSpeed)) 0.0 0.0) false false))

(fn ConstructionScript)